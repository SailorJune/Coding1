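; BP_Item is an item actor that sets its stats by type and damages an enemy when play begins.
; Constructor, called from BeginPlay, randomizes damage and picks an unset name for weapons, while tools and consumables get fixed damage.
; After printing the stats and a short delay, Attack subtracts Damage from the Health of the BP_Enemy found by GetActorOfClass.
; A Timeline also animates the Cube's relative Z location.
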(event EventBeginPlay
  (Utilities|FlowControl|Sequence
    (:then_0
      (CallFunction|Constructor)
      (Development|PrintString (Utilities|String|Append "Name" (Variables|Default|GetName) "Damage" (Utilities|String|ToString(Integer) (Variables|Default|GetDamage))) true true "(R=0.000000,G=0.660000,B=1.000000,A=1.000000)" 4e+01)
      (Utilities|FlowControl|Delay 0.2)
      (bind _returnvalue (Actor|GetActorOfClass "/Game/Blueprints/BP_Enemy.BP_Enemy_C"))
      (CallFunction|Attack _returnvalue))
    (:then_1
      (bind _newtrack_0 (Timeline|Timeline Play)
        (:Update
          (Transformation|SetRelativeLocation (Variables|Default|GetCube) (Math|Vector|MakeVector 0.0 0.0 (Math|Float|Lerp 0.0 1e+02 _newtrack_0)) false false))))))

(event Collision|EventActorBeginOverlap
  (params (OtherActor :type Actor%20Object%20Reference)))

(event EventTick
  (params (DeltaSeconds :type Float%20%28single-precision%29)))

(fn ConstructionScript)

(fn Constructor
  (bind _weaponsnames (Variables|Default|GetweaponsNames))
  (switch Utilities|FlowControl|Switch|SwitchonItemType (Variables|Default|GetType)
    (:NewEnumerator0
      (Variables|Default|SetDamage (Math|Random|RandomIntegerinRange 3 6))
      (if (Utilities|Enum|Equal(Enum) (Variables|Default|GetName) "")
        (Utilities|Array|Shuffle _weaponsnames)
        (Variables|Default|SetName (Utilities|Array|Get(acopy) _weaponsnames))))
    (:NewEnumerator2
      (Variables|Default|SetDamage 1))
    (:NewEnumerator3
      (Variables|Default|SetDamage 0))))

(fn Attack
  (params (Given%20Enemy :type BP%20Enemy%20Object%20Reference))
  (Variables|/Game/Blueprints/BP_Enemy.BP_Enemy_C|SetHealth Given%20Enemy (- (Variables|/Game/Blueprints/BP_Enemy.BP_Enemy_C|GetHealth Given%20Enemy) (Variables|Default|GetDamage))))