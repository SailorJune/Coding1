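; BP_Enemy is an enemy actor that dies when the third-person player character overlaps its capsule.
; The overlap sets Health below zero rather than destroying the actor directly.
; A self-calling CheckHealth event, started on BeginPlay, polls Health on a short delay, then destroys the actor and prints a red debug scream once it is negative.
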(event OnComponentBeginOverlap(Capsule)
  (params (OverlappedComponent :type Primitive%20Component%20Object%20Reference) (OtherActor :type Actor%20Object%20Reference) (OtherComp :type Primitive%20Component%20Object%20Reference) (OtherBodyIndex :type Integer) (bFromSweep :type Boolean) (SweepResult :type Hit%20Result%20Structure%20%28by%20ref%29))
  (Utilities|Casting|CastToBP_ThirdPersonCharacter OtherActor)
  (Variables|Default|SetHealth -1.0))

(event Custom|Check%20Health
  (Utilities|FlowControl|Delay 0.2)
  (if (>= (Variables|Default|GetHealth) 0.0)
    (CallFunction|CheckHealth)
    (else
      (Actor|DestroyActor)
      (Development|PrintString "AAAAAAAAAAAAA" true true "(R=1.000000,G=0.013417,B=0.000000,A=1.000000)"))))

(event EventBeginPlay
  (CallFunction|CheckHealth))

(fn ConstructionScript)