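; BP_FunctionExploration is a practice Blueprint that explores functions and custom events by printing colored debug text on BeginPlay.
; It loops over the Names array twice, first in random colors and then colored by string length through GetColorByLegnth.
; A final loop sums random integer pairs with AddTwoColors, which colors each result by sign.
; The Say event handles these prints, treating magenta as a sentinel for a random color.
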(event Custom|say
  (params (InString :type String) (TextColor :type Linear%20Color%20Structure :default "(R=1.000000,G=0.000000,B=1.000000,A=1.000000)"))
  ;[1 1 1] Print This SHit
  (if (== TextColor "(R=1.000000,G=0.000000,B=1.000000,A=1.000000)")
    (Development|PrintString InString true true (Utilities|Struct|MakeLinearColor (Math|Random|RandomFloat) (Math|Random|RandomFloat) (Math|Random|RandomFloat) 1.0) 8.0)
    (else
      (Development|PrintString InString true true TextColor 8.0))))

(event EventBeginPlay
  (bind _names (Variables|Default|GetNames))
  ;[1 1 1] Print array
  (Development|PrintString "Hello")
  (for _array_element _names
    (CallFunction|Say _array_element "(R=1.000000,G=0.000000,B=1.000000,A=1.000000)"))
  ;[1 0 0.5384] Random Color
  (for _array_element_2 _names
    (bind _output (CallFunction|GetColorbyLegnth _array_element_2))
    (CallFunction|Say _array_element_2 _output))
  ;[1 0 0] Add Random Numbers and Print Colors
  (for _index (range 0 9)
    (bind (_sum _color) (CallFunction|AddTwoColors (Math|Random|RandomIntegerinRange -10 10) (Math|Random|RandomIntegerinRange -10 10)))
    (CallFunction|Say (Utilities|String|ToString(Integer) _sum) _color)))

(event Collision|EventActorBeginOverlap
  (params (OtherActor :type Actor%20Object%20Reference)))

(event EventTick
  (params (DeltaSeconds :type Float%20%28single-precision%29)))

(fn ConstructionScript)

(fn GetColorbyLegnth
  (params (Input :type String))
  (bind _returnvalue (Utilities|String|Len Input))
  (bind _returnvalue_2 (- _returnvalue 5))
  (bind _returnvalue_3 (* _returnvalue_2 0.2))
  (if (<= _returnvalue 5)
    (LocalVariables|SetOutputColor "(R=1.000000,G=0.000000,B=0.068657,A=1.000000)")
    (elif (>= _returnvalue 10)
      (LocalVariables|SetOutputColor "(R=0.000000,G=0.152652,B=1.000000,A=1.000000)")
      (else
        (LocalVariables|SetOutputColor (Utilities|Struct|MakeLinearColor _returnvalue_3 _returnvalue_3 _returnvalue_3 1.0)))))
  (return (LocalVariables|GetOutputColor)))

(fn AddTwoColors
  (params (First%20Num :type Integer) (Second%20Num :type Integer))
  (bind _returnvalue (+ First%20Num Second%20Num))
  (if (>= _returnvalue 0)
    (LocalVariables|SetColorLocal "(R=0.000000,G=1.000000,B=0.000000,A=1.000000)")
    (else
      (LocalVariables|SetColorLocal "(R=1.000000,G=0.000000,B=0.000000,A=1.000000)")))
  (return _returnvalue (LocalVariables|GetColorLocal)))