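; BP_EnemySpawner populates the level with BP_Enemy actors and respawns a new batch whenever none remain.
; On BeginPlay it gathers all BP_EnemySpawnLocation actors and prints their count.
; SpawnEnemies gives each location a weighted random chance to spawn an enemy at its transform.
; CheckEenemyCount then polls for living BP_Enemy actors by re-calling itself after a short Delay, triggering SpawnEnemies when the count hits zero.
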(event Custom|SpawnEnemies
  ;[0 1 0.1981] Run Spawn Enemies > Randomize chance of spawning enemies > spawn enemy
  (for _array_element (stale EventBeginPlay _outactors)
    (if (< (Math|Random|RandomFloat) 0.8)
      (Game|SpawnActorfromClass "/Game/Blueprints/BP_Enemy.BP_Enemy_C" (Transformation|GetActorTransform _array_element) "Undefined" "MultiplyWithRoot" 0 0))))

(event Custom|check%20eenemy%20count
  ;[0.6191 1 0.2103] Check for 0 enemies remaining > Loop
  (bind _outactors (Actor|GetAllActorsOfClass "/Game/Blueprints/BP_Enemy.BP_Enemy_C"))
  (if (> (Utilities|Array|Length _outactors) 0)
    _
    (else
      (CallFunction|SpawnEnemies)))
  (Utilities|FlowControl|Delay 0.2)
  (CallFunction|CheckEenemyCount))

(event EventBeginPlay
  ;[0 1 0.7335] Start > Get no. of Enemy spawner > Run Spawn
  (bind _outactors (Actor|GetAllActorsOfClass "/Game/Blueprints/BP_EnemySpawnLocation.BP_EnemySpawnLocation_C"))
  (Development|PrintString (Utilities|String|Append "There are " (Utilities|String|ToString(Integer) (Utilities|Array|Length _outactors)) " spawn locations") true true "(R=0.000000,G=0.660000,B=1.000000,A=1.000000)" 1e+01)
  (CallFunction|SpawnEnemies)
  (CallFunction|CheckEenemyCount))

(fn ConstructionScript)